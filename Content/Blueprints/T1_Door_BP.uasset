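; T1_Door_BP is a key-locked sliding door Blueprint, bundling the door with its key pickup.
; Overlapping the key's box sets HastheKey and destroys the key, whose box is positioned from KeyLocation in the construction script.
; Door-box begin and end overlaps share a FlipFlop that alternately plays a sliding Timeline or reverses it after a delay.
; Without the key, either overlap prints a reminder.
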(event OnComponentBeginOverlap(Box)
  (params (OverlappedComponent :type Primitive%20Component%20Object%20Reference) (OtherActor :type Actor%20Object%20Reference) (OtherComp :type Primitive%20Component%20Object%20Reference) (OtherBodyIndex :type Integer) (bFromSweep :type Boolean) (SweepResult :type Hit%20Result%20Structure%20%28by%20ref%29))
  ;[0.5349 1 0.5662] Slide the Door
  (if (Variables|Default|GetHastheKey?)
    (Utilities|FlowControl|FlipFlop
      (:A
        (bind _speed (Timeline|Timeline Play)
          (:Update
            (Transformation|SetRelativeLocation (Variables|Default|GetDoor) (Math|Vector|Lerp(Vector) "0, 0, 0" "200.000000,0.000000,0.000000" _speed) false false))))
      (:B
        (Utilities|FlowControl|Delay 3.0)
        (Timeline|Timeline Reverse)))
    (else
      (Development|PrintString "No Key, Please get the key first"))))

(event OnComponentEndOverlap(Box)
  (params (OverlappedComponent :type Primitive%20Component%20Object%20Reference) (OtherActor :type Actor%20Object%20Reference) (OtherComp :type Primitive%20Component%20Object%20Reference) (OtherBodyIndex :type Integer))
  ;[0.5349 1 0.5662] Slide the Door
  (if (Variables|Default|GetHastheKey?)
    (Utilities|FlowControl|FlipFlop
      (:A
        (bind _speed (Timeline|Timeline Play)
          (:Update
            (Transformation|SetRelativeLocation (Variables|Default|GetDoor) (Math|Vector|Lerp(Vector) "0, 0, 0" "200.000000,0.000000,0.000000" _speed) false false))))
      (:B
        (Utilities|FlowControl|Delay 3.0)
        (Timeline|Timeline Reverse)))
    (else
      (Development|PrintString "No Key, Please get the key first"))))

(event OnComponentBeginOverlap(Box_Key)
  (params (OverlappedComponent :type Primitive%20Component%20Object%20Reference) (OtherActor :type Actor%20Object%20Reference) (OtherComp :type Primitive%20Component%20Object%20Reference) (OtherBodyIndex :type Integer) (bFromSweep :type Boolean) (SweepResult :type Hit%20Result%20Structure%20%28by%20ref%29))
  ;[1 0.3698 0.3698] Get the Key
  (Variables|Default|SetHastheKey? true)
  (Utilities|FlowControl|Delay 0.2)
  (Components|DestroyComponent (Variables|Default|GetKey)))

(fn ConstructionScript
  (Transformation|SetRelativeLocation (Variables|Default|GetBox_Key) (Variables|Default|GetKeyLocation) false false))